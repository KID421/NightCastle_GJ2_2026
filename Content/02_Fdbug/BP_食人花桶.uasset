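; Piranha-plant pipe hazard that sends its plant out when the player character approaches and restarts the level when the player touches its hit volume.
; Entering the detection area stores the plant's position, then a timeline lerps it to an endpoint marker.
; Each timeline finish waits briefly, then a FlipFlop alternates playing from start and reversing from end, looping indefinitely.
; Hits restart through a console command; an OpenLevel call is left unconnected.
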(event `self.玩家偵測區域.OnComponentBeginOverlap`
  (params (OverlappedComponent :type "PrimitiveComponent Object Reference") (OtherActor :type "Actor Object Reference") (OtherComp :type "PrimitiveComponent Object Reference") (OtherBodyIndex :type Integer) (bFromSweep :type Boolean) (SweepResult :type "HitResult Structure (by ref)"))
  (cast `/Game/ThirdPerson/Blueprints/BP_ThirdPersonCharacter` OtherActor)
  (set `self.食人花原點` (`SceneComponent.K2_GetComponentLocation` (`self.食人花`)))
  (bind (_direction `_食人花伸縮`) (`Timeline|食人花伸出` :!label _label)
    (:`Update`
      (`SceneComponent.K2_SetWorldLocation` (`self.食人花`) (`KismetMathLibrary.VLerp` (`self.食人花原點`) (`SceneComponent.K2_GetComponentLocation` (`self.食人花移動終點`)) `_食人花伸縮`) false false))
    (:`Finished`
      (`KismetSystemLibrary.Delay` 0.8)
      (`/Engine/EditorBlueprintResources/StandardMacros.FlipFlop`
        (:`A`
          (goto _label :!via `PlayFromStart`))
        (:`B`
          (goto _label :!via `ReverseFromEnd`))))))

(event `self.撞擊判定.OnComponentBeginOverlap`
  (params (OverlappedComponent :type "PrimitiveComponent Object Reference") (OtherActor :type "Actor Object Reference") (OtherComp :type "PrimitiveComponent Object Reference") (OtherBodyIndex :type Integer) (bFromSweep :type Boolean) (SweepResult :type "HitResult Structure (by ref)"))
  (cast `/Game/ThirdPerson/Blueprints/BP_ThirdPersonCharacter` OtherActor)
  (`KismetSystemLibrary.PrintText` "Hello")
  (`KismetSystemLibrary.ExecuteConsoleCommand` "RestartLevel" null))

(fn `UserConstructionScript`)