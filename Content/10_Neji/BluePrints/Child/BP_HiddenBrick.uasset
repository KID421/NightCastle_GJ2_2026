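; BP_HiddenBrick is a child brick Blueprint that stays invisible until it is hit.
; On BeginPlay it hides the brick mesh, Decal and ForDecal components through the shared SetObjVisible helper.
; OnBrickHit shows them again and plays a 2D reveal sound.
; SetObjVisible changes only visibility, without propagating to children or touching collision.
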(event `self.ReceiveBeginPlay`
  (`self.SetObjVisible` false))

(fn `OnBrickHit`
  (params (PlayerBP :type "/Game/ThirdPerson/Blueprints/BP_ThirdPersonCharacter Object Reference"))
  (`self.SetObjVisible` true)
  (`GameplayStatics.PlaySound2D` "/Game/10_Neji/SFX/Sound_HiddenBrick.Sound_HiddenBrick" 1.0 1.0 0.0 null null))

(fn `SetObjVisible`
  (params (Visible :type Boolean))
  (`SceneComponent.SetVisibility` (`self.BrickMesh`) Visible false)
  (`SceneComponent.SetVisibility` (`self.Decal`) Visible false)
  (`SceneComponent.SetVisibility` (`self.ForDecal`) Visible false))

(fn `UserConstructionScript`
  (`parent.UserConstructionScript`))