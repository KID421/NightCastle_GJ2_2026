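; BP_TrapFloor is a breakable floor trap with a death zone that restarts the level.
; When the third-person character overlaps the Box trigger, the Cube is destroyed with a brick-shattering sound.
; Any overlap with DeadZone fires once, playing a scream sound, waiting briefly, then reopening the current level by name.
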(event `self.Box.OnComponentBeginOverlap`
  (params (OverlappedComponent :type "PrimitiveComponent Object Reference") (OtherActor :type "Actor Object Reference") (OtherComp :type "PrimitiveComponent Object Reference") (OtherBodyIndex :type Integer) (bFromSweep :type Boolean) (SweepResult :type "HitResult Structure (by ref)"))
  (bind _cube (`self.Cube`))
  ; Hide Cube
  (cast `/Game/ThirdPerson/Blueprints/BP_ThirdPersonCharacter` OtherActor)
  (`/Engine/EditorBlueprintResources/StandardMacros.IsValid` _cube
    (:`Is Valid`
      (`ActorComponent.K2_DestroyComponent` _cube)
      (`GameplayStatics.PlaySound2D` "/Game/02_Fdbug/音效/音效_磚塊碎裂.音效_磚塊碎裂" 1.0 1.0 0.0 null null))))

(event `self.DeadZone.OnComponentBeginOverlap`
  (params (OverlappedComponent :type "PrimitiveComponent Object Reference") (OtherActor :type "Actor Object Reference") (OtherComp :type "PrimitiveComponent Object Reference") (OtherBodyIndex :type Integer) (bFromSweep :type Boolean) (SweepResult :type "HitResult Structure (by ref)"))
  ; Restart Game
  (`/Engine/EditorBlueprintResources/StandardMacros.DoOnce` false
    (:`Completed`
      (`GameplayStatics.PlaySound2D` "/Game/05_FunGame/ahhhhh-meme-made-with-Voicemod.ahhhhh-meme-made-with-Voicemod" 1.0 1.0 0.0 null null)
      (`KismetSystemLibrary.Delay` 3.0)
      (bind _returnvalue (`GameplayStatics.GetCurrentLevelName` true))
      (`GameplayStatics.OpenLevel` (`KismetStringLibrary.Conv_StringToName` _returnvalue)))))

(fn `UserConstructionScript`)