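; BP_CoinCS is a coin pickup Blueprint that builds on overlap and deletion behavior from its parent class.
; On player overlap it calls AddResourceMessage on the player actor with a value of zero.
; Its DeleteActor override calls the parent implementation, then plays a 2D coin sound and prints a "Coin" debug string.
; BeginPlay, overlap and Tick event stubs are disabled.
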(event `/Game/08_Aylmer/Main/Interface/BPI_Interact.OnPlayerOverlap`
  (params (PlayerActor :type "Actor Object Reference"))
  (message `/Game/08_Aylmer/Main/Interface/BPI_Interact.AddResource` PlayerActor 0))

(fn `DeleteActor`
  (params (Actor :type "Actor Object Reference"))
  (`parent.DeleteActor` Actor)
  (`GameplayStatics.PlaySound2D` "/Game/06_Yayi/soundEffect/coin.coin" 1.0 1.0 0.0 null null)
  (`KismetSystemLibrary.PrintString` "Coin"))

(fn `UserConstructionScript`
  (`parent.UserConstructionScript`))