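; A Mario-style question block that releases a mushroom pickup the first time the third-person character overlaps its Rock component.
; The hit also swaps the block's material and plays a brick-breaking sound.
; The spawned BP_蘑菇 starts without collision or physics while a timeline lifts it from the block's position.
; When the timeline finishes, the mushroom becomes edible and regains physics and collision.
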(event `self.Rock.OnComponentBeginOverlap`
  (params (OverlappedComponent :type "PrimitiveComponent Object Reference") (OtherActor :type "Actor Object Reference") (OtherComp :type "PrimitiveComponent Object Reference") (OtherBodyIndex :type Integer) (bFromSweep :type Boolean) (SweepResult :type "HitResult Structure (by ref)"))
  (cast `/Game/ThirdPerson/Blueprints/BP_ThirdPersonCharacter` OtherActor)
  (`/Engine/EditorBlueprintResources/StandardMacros.DoOnce` false
    (:`Completed`
      (`self.生出蘑菇`)
      (`PrimitiveComponent.SetMaterial` (`self.Rock`) 0 "/Engine/MaterialTemplates/VertexAnimation/AdvancedFlag.AdvancedFlag")
      (`GameplayStatics.PlaySound2D` "/Game/02_Fdbug/音效/音效_磚塊碎裂.音效_磚塊碎裂" 1.0 1.0 0.0 null null))))

(event `生出蘑菇`
  (bind `_蘑菇本人` (`self.蘑菇本人`))
  (bind _sphere (`/Game/06_Yayi/BP_蘑菇.Sphere` `_蘑菇本人`))
  ; 事件：生成蘑菇
  (bind _returnvalue (`|SpawnActorFromClass` "/Game/06_Yayi/BP_蘑菇.BP_蘑菇_C" (`SceneComponent.K2_GetComponentToWorld` (`self.Rock`)) "Undefined" "MultiplyWithRoot" null true null))
  (bind _output_get (set `self.蘑菇本人` _returnvalue))
  (bind _sphere_2 (`/Game/06_Yayi/BP_蘑菇.Sphere` _output_get))
  (`PrimitiveComponent.SetCollisionEnabled` _sphere_2 "NoCollision")
  (`PrimitiveComponent.SetSimulatePhysics` _sphere_2 false)
  (`KismetSystemLibrary.PrintString` "生出蘑菇！")
  (bind (_direction `_蘑菇座標`) (`Timeline|生成蘑菇` :!via `PlayFromStart`)
    (:`Update`
      (`self.K2_SetActorLocation` `_蘑菇本人` (`KismetMathLibrary.MakeVector` (.x (.location (`SceneComponent.K2_GetComponentToWorld` (`self.Rock`)))) (.y (.location (`SceneComponent.K2_GetComponentToWorld` (`self.Rock`)))) (+ `_蘑菇座標` (.z (.location (`SceneComponent.K2_GetComponentToWorld` (`self.Rock`)))))) false false))
    (:`Finished`
      (set `/Game/06_Yayi/BP_蘑菇.給不給吃` true `_蘑菇本人`)
      (`PrimitiveComponent.SetSimulatePhysics` _sphere true)
      (`PrimitiveComponent.SetCollisionEnabled` _sphere "QueryAndPhysics"))))

(fn `UserConstructionScript`)