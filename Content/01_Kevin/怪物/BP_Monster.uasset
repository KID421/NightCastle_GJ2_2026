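; BP_Monster is a patrolling enemy that restarts the level when its box overlaps the player character.
; From BeginPlay it loops AI MoveTo between PointA and PointB, pausing after each successful arrival.
; Its Monster_Been_Crush event handles death by destroying the actor, playing a stomp sound and printing a debug message.
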(event `self.Box.OnComponentBeginOverlap`
  (params (OverlappedComponent :type "PrimitiveComponent Object Reference") (OtherActor :type "Actor Object Reference") (OtherComp :type "PrimitiveComponent Object Reference") (OtherBodyIndex :type Integer) (bFromSweep :type Boolean) (SweepResult :type "HitResult Structure (by ref)"))
  (cast `/Game/ThirdPerson/Blueprints/BP_ThirdPersonCharacter` OtherActor)
  (`KismetSystemLibrary.PrintText` "Hello")
  (`KismetSystemLibrary.ExecuteConsoleCommand` "RestartLevel" null))

(event `self.ReceiveBeginPlay`
  (bind _pointb (`self.PointB`))
  (bind _pointa (`self.PointA`))
  (if (not (and (`KismetSystemLibrary.IsValid` _pointa) (`KismetSystemLibrary.IsValid` _pointb)))
    (`KismetSystemLibrary.Delay` 2.0))
  (`|AIMoveTo` self (`self.K2_GetActorLocation` _pointa) null :!label _label
    (:`OnSuccess`
      (`KismetSystemLibrary.Delay` 2.0)
      (`|AIMoveTo` self (`self.K2_GetActorLocation` _pointb) null
        (:`OnSuccess`
          (`KismetSystemLibrary.Delay` 1.0)
          (goto _label))))))

(event `Monster_Been_Crush`
  (`self.K2_DestroyActor`)
  (`GameplayStatics.PlaySound2D` "/Game/02_Fdbug/音效/音效_踩死怪物.音效_踩死怪物" 1.0 1.0 0.0 null null)
  (`KismetSystemLibrary.PrintText` "ByeBye"))

(fn `UserConstructionScript`)