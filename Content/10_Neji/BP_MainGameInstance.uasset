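; Game instance that holds the player's stats and handles game over, level restart and level loading.
; Game over fires the OnStatsUpdateRequested dispatcher, shows the 遊戲結束 (game over) widget and switches to UI-only input with a visible cursor.
; Stats are replaced wholesale through UpdateStats, while reset and restart restore health to its default, with restart also running the RestartLevel console command.
; Helper functions open levels by name or object reference.
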(fn `GameOverFunc`
  (bind _returnvalue (`GameplayStatics.GetPlayerController` 0))
  (`self.OnStatsUpdateRequested`)
  (bind _returnvalue_2 (`|CreateWidget` "/Game/07_Leo/WB_遊戲結束.WB_遊戲結束_C"))
  (`UserWidget.AddToViewport` _returnvalue_2 0)
  (`WidgetBlueprintLibrary.SetInputMode_UIOnlyEx` _returnvalue null)
  (set `PlayerController.bShowMouseCursor` true _returnvalue))

(fn `LoadLevelByName`
  (params (LevelName :type Name))
  (`GameplayStatics.OpenLevel` LevelName))

(fn `LoadLevelByObject`
  (params (Level :type "World Soft Object Reference"))
  (`GameplayStatics.OpenLevelBySoftObjectPtr` Level))

(fn `ResetStats`
  (setmembers `/Game/08_Aylmer/Main/Structure/S_CharacterStats` :`StructRef` (`self.PlayerStats`) :`CurrentState` "NewEnumerator0" :`Health` (`self.DefaultHealth`) :`CoinCount` 0 :`Score` 0))

(fn `RestartLevel`
  (setmembers `/Game/08_Aylmer/Main/Structure/S_CharacterStats` :`StructRef` (`self.PlayerStats`) :`Health` (`self.DefaultHealth`))
  (`KismetSystemLibrary.ExecuteConsoleCommand` "RestartLevel" null))

(fn `UpdateStats`
  (params (NewStat :type "/Game/08_Aylmer/Main/Structure/S_CharacterStats Structure"))
  (set `self.PlayerStats` NewStat))