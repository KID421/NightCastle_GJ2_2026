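; BP_CoinBrick is a child brick Blueprint that gives the player coins on repeated hits within a time window.
; The first hit opens the window by setting CanHit and starting a WaitTime timer, whose EndHit event clears the flag.
; Each hit from a valid player calls GetCoin, so the first hit after the window closes still pays a coin before OnBrickDisabled runs.
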(event `OnFirstHit`
  ; 第一次撞擊後開始計時
  (set `self.CanHit` true)
  (`KismetSystemLibrary.K2_SetTimerDelegate` (delegate `EndHit`) (`self.WaitTime`))
  (set `self.HitStarted` true))

(event `EndHit`
  ; 停止碰撞
  (set `self.CanHit` false))

(fn `OnBrickHit`
  (params (PlayerBP :type "/Game/ThirdPerson/Blueprints/BP_ThirdPersonCharacter Object Reference"))
  (`/Engine/EditorBlueprintResources/StandardMacros.IsValid` PlayerBP
    (:`Is Valid`
      (if (not (`self.HitStarted`))
        (`self.OnFirstHit`))
      (`/Game/ThirdPerson/Blueprints/BP_ThirdPersonCharacter.GetCoin` PlayerBP)
      (if (not (`self.CanHit`))
        (`self.OnBrickDisabled`)))))

(fn `UserConstructionScript`
  (`parent.UserConstructionScript`))