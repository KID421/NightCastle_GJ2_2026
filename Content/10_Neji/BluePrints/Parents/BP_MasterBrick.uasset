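; Parent Blueprint for hittable bricks, providing shared hit, coin pop and break behavior.
; A block hit forwards the player to OnBrickHit, which is empty here.
; SpawnCoin spawns an uncollectable coin at the brick, offsets its height through a timeline scaled by CoinHeight, then destroys it when finished.
; OnBrickDisabled destroys the brick and plays a shattering sound.
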(event `/Game/10_Neji/BluePrints/Interfaces/BPI_BlockAction.OnBlockHit`
  (params (PlayerBP :type "/Game/ThirdPerson/Blueprints/BP_ThirdPersonCharacter Object Reference"))
  (`self.OnBrickHit` PlayerBP))

(event `SpawnCoin`
  (bind _returnvalue_location (`KismetMathLibrary.BreakTransform` (`self.GetTransform`)))
  (bind (_returnvalue_x _returnvalue_y _returnvalue_z) (`KismetMathLibrary.BreakVector` (`self.K2_GetActorLocation`)))
  (bind _returnvalue (`|SpawnActorFromClass` "/Game/06_Yayi/BP_Coin.BP_Coin_C" (`KismetMathLibrary.MakeTransform` _returnvalue_location (struct :`Yaw` 90.0)) "Undefined" "MultiplyWithRoot" null true null))
  (bind (_direction _duration) (`Timeline|CoinSpawnMovement` :!via `PlayFromStart`)
    (:`Update`
      (`self.K2_SetActorLocation` _returnvalue (`KismetMathLibrary.MakeVector` _returnvalue_x _returnvalue_y (+ _returnvalue_z (* _duration (`self.CoinHeight`)))) false false))
    (:`Finished`
      (`self.K2_DestroyActor` _returnvalue))))

(fn `OnBrickDisabled`
  (`self.K2_DestroyActor`)
  (`GameplayStatics.PlaySound2D` "/Game/02_Fdbug/音效/音效_磚塊碎裂.音效_磚塊碎裂" 1.0 1.0 0.0 null null))

(fn `OnBrickHit`
  (params (PlayerBP :type "/Game/ThirdPerson/Blueprints/BP_ThirdPersonCharacter Object Reference")))

(fn `UserConstructionScript`)