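; BP_蘑菇 is a mushroom pickup that raises the third-person character's health (血量) by one.
; When the character overlaps its sphere and the edible flag (給不給吃) is on, it increments health, plays an eating sound and destroys itself.
; With both that flag and the auto-move flag (要不要自動移動) on, Tick slides it along world X by a fixed, unswept step each frame, independent of delta time.
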(event `self.Sphere.OnComponentBeginOverlap`
  (params (OverlappedComponent :type "PrimitiveComponent Object Reference") (OtherActor :type "Actor Object Reference") (OtherComp :type "PrimitiveComponent Object Reference") (OtherBodyIndex :type Integer) (bFromSweep :type Boolean) (SweepResult :type "HitResult Structure (by ref)"))
  (bind _asbp_third_person_character (cast `/Game/ThirdPerson/Blueprints/BP_ThirdPersonCharacter` OtherActor))
  (if (`self.給不給吃`)
    (`/Engine/EditorBlueprintResources/StandardMacros.IncrementInt` (`/Game/ThirdPerson/Blueprints/BP_ThirdPersonCharacter.血量` _asbp_third_person_character)
      (:`  `
        (`GameplayStatics.PlaySound2D` "/Game/06_Yayi/soundEffect/eatMushroom.eatMushroom" 1.0 1.0 0.0 null null)
        (`self.K2_DestroyActor`)))))

(event `self.ReceiveTick`
  (params (DeltaSeconds :type "Float (single-precision)"))
  (if (and (`self.要不要自動移動`) (`self.給不給吃`))
    (`self.K2_AddActorWorldOffset` (10.0 0.0 0.0))))

(fn `UserConstructionScript`)